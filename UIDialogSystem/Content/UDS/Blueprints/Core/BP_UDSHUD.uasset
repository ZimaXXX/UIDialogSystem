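; BP_UDSHUD is the HUD for the UDS dialogue system, showing its UI and handling dialogue skip input.
; On BeginPlay it enables input from the first player controller, then creates the WBP_UDSHUD widget, stores it and adds it to the viewport.
; The IA_UI_Skip Enhanced Input action calls the UDSDialogueManagerSubsystem to skip the current dialogue.
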(event Input|EnhancedActionEvents|EnhancedInputActionIA_UI_Skip
  (params (ActionValue :type Boolean) (ElapsedSeconds :type Float%20%28double-precision%29) (TriggeredSeconds :type Float%20%28double-precision%29) (InputAction :type Input%20Action%20Object%20Reference :default "/Game/ThirdPerson/Input/Actions/IA_UI_Skip.IA_UI_Skip"))
  (Class|UDSDialogueManagerSubsystem|SkipCurrentDialogue (Subsystems|GetUDSDialogueManagerSubsystem)))

(event EventBeginPlay
  (|CallParentFunction)
  (Utilities|FlowControl|Sequence
    (:then_0
      (Input|EnableInput (Game|GetPlayerController 0)))
    (:then_1
      (bind _returnvalue (UserInterface|CreateWidget "/Game/UDS/Blueprints/Widgets/WBP_UDSHUD.WBP_UDSHUD_C" (Game|GetPlayerController 0)))
      (bind _output_get (Variables|Default|SetWBP_HUD _returnvalue))
      (UserInterface|Viewport|AddtoViewport _output_get 0))))

(fn ConstructionScript)